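; Gameplay game mode that handles team-based character spawning for attackers and defenders.
; RequestSpawn branches on team, spawning an attacker for Team A or a defender for Team B at a random PlayerStart, with no team filtering of start points.
; It sets the pawn's team, has the requesting controller possess it, and adds it uniquely to the Players list in BP_GameplayGameState.
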(event `RequestSpawn`
  (params (Team :type "/Game/Blueprints/TutoMulti/Team Enum" :default "NewEnumerator0") (Controller :type "Controller Object Reference"))
  (bind _players (`/Game/Blueprints/BP_GameplayGameState.Players` (cast `/Game/Blueprints/BP_GameplayGameState` (`GameplayStatics.GetGameState`) :!pure true)))
  (switch `/Game/Blueprints/TutoMulti/Team` Team
    (:`NewEnumerator1`
      (bind _outactors (`GameplayStatics.GetAllActorsOfClass` "/Script/Engine.PlayerStart"))
      (bind _returnvalue (`|SpawnActorFromClass` "/Game/ThirdPersonCPP/Blueprints/YTCharacter_Attacker.YTCharacter_Attacker_C" (`self.GetTransform` (`|GetArrayItem` _outactors (`KismetMathLibrary.RandomInteger` (`KismetArrayLibrary.Array_Length` _outactors)))) "AdjustIfPossibleButAlwaysSpawn" "OverrideRootScale" null 0 Team null))
      (`Controller.Possess` Controller _returnvalue)
      (`KismetArrayLibrary.Array_AddUnique` _players _returnvalue))
    (:`NewEnumerator2`
      (bind _outactors_2 (`GameplayStatics.GetAllActorsOfClass` "/Script/Engine.PlayerStart"))
      (bind _returnvalue_2 (`|SpawnActorFromClass` "/Game/ThirdPersonCPP/Blueprints/YTCharacter_Defender.YTCharacter_Defender_C" (`self.GetTransform` (`|GetArrayItem` _outactors_2 (`KismetMathLibrary.RandomInteger` (`KismetArrayLibrary.Array_Length` _outactors_2)))) "AdjustIfPossibleButAlwaysSpawn" "OverrideRootScale" null 0 Team null))
      (`Controller.Possess` Controller _returnvalue_2)
      (`KismetArrayLibrary.Array_AddUnique` _players _returnvalue_2))))

(fn `UserConstructionScript`)