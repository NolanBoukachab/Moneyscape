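; BP_GameplayController is a player controller that handles team selection and spawn requests for gameplay.
; On begin play, the server possesses the first CameraSOG actor found in the level, while the local client adds the MyTeamSelection and InGame_WB widgets and shows the mouse cursor.
; TeamSelected forwards the chosen team and itself to BP_GameplayGameMode's RequestSpawn.
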(event `self.ReceiveBeginPlay`
  (`|ExecutionSequence`
    (:`then_0`
      (`/Engine/EditorBlueprintResources/ActorMacros.Switch Has Authority`
        (:`Authority`
          (bind _outactors (`GameplayStatics.GetAllActorsOfClass` "/Game/Blueprints/TutoMulti/CameraSOG.CameraSOG_C"))
          (`self.Possess` (`|GetArrayItem` _outactors)))))
    (:`then_1`
      (if (`self.IsLocalController`)
        (bind _returnvalue (`|CreateWidget` "/Game/UI/TutoMulti/MyTeamSelection.MyTeamSelection_C"))
        (`UserWidget.AddToViewport` _returnvalue 0)
        (set `self.bShowMouseCursor` true)
        (bind _returnvalue_2 (`|CreateWidget` "/Game/UI/InGame_WB.InGame_WB_C"))
        (`UserWidget.AddToViewport` _returnvalue_2 0)))))

(event `self.ReceiveTick`
  (params (DeltaSeconds :type "Float (single-precision)")))

(event `TeamSelected`
  (params (Team :type "/Game/Blueprints/TutoMulti/Team Enum" :default "NewEnumerator0"))
  (`/Game/Blueprints/BP_GameplayGameMode.RequestSpawn` (cast `/Game/Blueprints/BP_GameplayGameMode` (`GameplayStatics.GetGameMode`) :!pure true) Team self))

(fn `UserConstructionScript`)