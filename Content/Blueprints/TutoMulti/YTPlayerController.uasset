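; Player controller for a multiplayer game that handles team selection before the player spawns.
; On BeginPlay the authority possesses the first CameraSOG actor found in the level, while the local controller shows the MyTeamSelection widget and mouse cursor.
; A team-selected event forwards the chosen team and this controller to YTGameMode's RequestSpawn, leaving spawning to the game mode.
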(event `self.ReceiveBeginPlay`
  (`|ExecutionSequence`
    (:`then_0`
      (`/Engine/EditorBlueprintResources/ActorMacros.Switch Has Authority`
        (:`Authority`
          (bind _outactors (`GameplayStatics.GetAllActorsOfClass` "/Game/Blueprints/TutoMulti/CameraSOG.CameraSOG_C"))
          (`self.Possess` (`|GetArrayItem` _outactors)))))
    (:`then_1`
      (if (`self.IsLocalController`)
        (bind _returnvalue (`|CreateWidget` "/Game/UI/TutoMulti/MyTeamSelection.MyTeamSelection_C"))
        (`UserWidget.AddToViewport` _returnvalue 0)
        (set `self.bShowMouseCursor` true)))))

(event `TeamSelectedeeee`
  (params (Team :type "/Game/Blueprints/TutoMulti/Team Enum" :default "NewEnumerator0"))
  (`/Game/Blueprints/TutoMulti/YTGameMode.RequestSpawn` (cast `/Game/Blueprints/TutoMulti/YTGameMode` (`GameplayStatics.GetGameMode`) :!pure true) Team self))

(fn `UserConstructionScript`)